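; Keypad code lock actor that shows a WB_TestWidget and flags itself unlocked when the correct password is entered.
; Key presses go through the local pawn's BP_InterfaceInteract RPC, since the lock is networked, with Interact as the entry point for each character.
; Each character is appended and checked, clearing a wrong full-length entry or updating the lock text on a match.
; Pressed buttons briefly flash on non-server instances only.
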(event Custom|RunInteract
  (params (Char :type Integer))
  (bind _output_get (Variables|Default|SetInterfaceComponent (Actor|GetComponentbyClass (Pawn|GetControlledPawn (Game|GetPlayerController 0)) "/Game/CodeLock/BP_InterfaceInteract.BP_InterfaceInteract_C")))
  (if (!= _output_get 0)
    (Default|InteractRPC _output_get Char self)))

(event Custom|Interact
  (params (Char :type Integer))
  (CallFunction|EnterPassword Char))

(event Custom|ChangeColor
  (params (Button :type Button%20Object%20Reference))
  (bind _widgetstyle (Variables|/Script/UMG.Button|GetWidgetStyle Button))
  (if (not (Networking|IsServer))
    (Class|Button|SetBackgroundColor Button (.specifiedcolor (.tintcolor (.pressed _widgetstyle))))
    (Utilities|FlowControl|Delay 0.2)
    (Class|Button|SetBackgroundColor Button (.specifiedcolor (.tintcolor (.normal _widgetstyle))))))

(event EventBeginPlay
  (bind _astest_widget (Utilities|Casting|CastToWB_TestWidget (UserInterface|GetUserWidgetObject (Variables|Default|GetWidget))))
  (bind _output_get (Variables|Default|SetAs%20Test%20Widget _astest_widget))
  (EventDispatchers|BindEventtoPasswordEntry _output_get (delegate Custom|RunInteract)))

(fn ConstructionScript)

(fn EnterPassword
  (params (Char :type Integer))
  (bind _as_test_widget (Variables|Default|GetAs%20Test%20Widget))
  (bind _textpassword (Variables|/Game/CodeLock/WB_TestWidget.WB_TestWidget_C|GetTextPassword _as_test_widget))
  (Variables|Default|SetCurrentPass (Utilities|String|Append (Utilities|String|ToString(Text) (Class|TextBlock|GetText _textpassword)) (Utilities|String|ToString(Integer) Char)))
  (Rendering|Components|TextRender|SetText _textpassword (Utilities|Text|ToText(String) (Variables|Default|GetCurrentPass)))
  (CallFunction|CheckPassword)
  (bind _button (Default|GetButtonfromIndex (Variables|Default|GetAs%20Test%20Widget) Char))
  (CallFunction|ChangeColor _button))

(fn CheckPassword
  (if (Utilities|Enum|Equal(Enum) (Variables|Default|GetCurrentPass) (Variables|Default|GetNeededPassword))
    (CallFunction|OpenLock)
    (elif (>= (Utilities|String|Len (Variables|Default|GetCurrentPass)) (Utilities|String|Len (Variables|Default|GetNeededPassword)))
      (bind _output_get (Variables|Default|SetCurrentPass ""))
      (Rendering|Components|TextRender|SetText (Variables|/Game/CodeLock/WB_TestWidget.WB_TestWidget_C|GetTextPassword (Variables|Default|GetAs%20Test%20Widget)) (Utilities|Text|ToText(String) _output_get)))))

(fn OpenLock
  (bind _as_test_widget (Variables|Default|GetAs%20Test%20Widget))
  (Variables|Default|SetUnlocked true)
  (Rendering|Components|TextRender|SetText (Variables|/Game/CodeLock/WB_TestWidget.WB_TestWidget_C|GetTextLocked _as_test_widget) "Unlocked")
  (Rendering|Components|TextRender|SetText (Variables|/Game/CodeLock/WB_TestWidget.WB_TestWidget_C|GetTextPassword _as_test_widget) "")
  (Variables|Default|SetCurrentPass ""))